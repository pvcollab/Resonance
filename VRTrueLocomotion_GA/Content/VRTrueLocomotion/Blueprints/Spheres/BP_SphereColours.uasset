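; BP_SphereColours is an actor in the VRTrueLocomotion Spheres folder that re-orients itself every frame using the player's camera rotation.
; On BeginPlay it finds and stores the BP_TrueLocomotionCharacter.
; Tick sets its rotation to look from its location toward the camera's forward vector, used directly as a world-space point without the camera location.
; It also prints that rotation as green debug text.
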(event `self.ReceiveBeginPlay`
  (bind _returnvalue (`GameplayStatics.GetActorOfClass` "/Game/VRTrueLocomotion/Blueprints/BP_TrueLocomotionCharacter.BP_TrueLocomotionCharacter_C"))
  (set `self.PlayerRef` _returnvalue))

(event `self.ReceiveTick`
  (params (DeltaSeconds :type "Float (single-precision)"))
  (bind _returnvalue (`KismetMathLibrary.FindLookAtRotation` (`self.K2_GetActorLocation`) (`KismetMathLibrary.Conv_RotatorToVector` (`SceneComponent.K2_GetComponentRotation` (`/Game/VRTrueLocomotion/Blueprints/BP_TrueLocomotionCharacter.PlayerCamera` (`self.PlayerRef`))))))
  (`self.K2_SetActorRotation` _returnvalue)
  (`KismetSystemLibrary.PrintString` (`KismetStringLibrary.Conv_RotatorToString` _returnvalue) true true (struct :`R` 0.078005 :`G` 1.0 :`A` 1.0)))

(fn `UserConstructionScript`)