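; BP_DemoDoor is a VR demo door that plays open and close animations on a skeletal mesh and toggles its collision.
; When the button option is enabled, BeginPlay caches the W_DoorActivator widget.
; Tick polls that widget's open flag and, if the player is allowed, opens the door through a DoOnce.
; Closing is a separate custom event with no caller in this graph.
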(event `self.ReceiveBeginPlay`
  ;[1 1 1] References Door Widget Opener on BeginPlay
  (if (`self.ShouldUseDoorButton`)
    (bind _asw_door_activator (cast `/Game/VRTrueLocomotion/Blueprints/Widgets/W_DoorActivator` (`WidgetComponent.GetUserWidgetObject` (`self.W_DoorButton`))))
    (set `self.DoorOpenerRef` _asw_door_activator)))

(event `self.ReceiveTick`
  (params (DeltaSeconds :type "Float (single-precision)"))
  (bind _dooropenerref (`self.DoorOpenerRef`))
  ;[1 1 1] Checks to See if Widget Has Been Hit and Opens Door
  (`/Engine/EditorBlueprintResources/StandardMacros.IsValid` _dooropenerref
    (:`Is Valid`
      (if (`/Game/VRTrueLocomotion/Blueprints/Widgets/W_DoorActivator.ShouldOpenDoor` _dooropenerref)
        (if (`self.CanPlayerOpenDoor`)
          (`/Engine/EditorBlueprintResources/StandardMacros.DoOnce` false
            (:`Completed`
              (`self.CE_OpenDoor`))))))))

(event `CE_OpenDoor`
  ;[1 1 1] Plays Door Anim When Called/ Updates Door State
  (if (not (`self.IsDoorOpen`))
    (`SkeletalMeshComponent.PlayAnimation` (`self.DoorSK`) "/Game/VRTrueLocomotion/Meshes/Door/Anim_DoorOpen.Anim_DoorOpen" false)
    (set `self.IsDoorOpen` true)
    (`PrimitiveComponent.SetCollisionResponseToAllChannels` (`self.DoorSK`) "ECR_Ignore")))

(event `CE_ClosesDoor`
  ;[1 1 1] Closes Door/Updates State
  (if (`self.IsDoorOpen`)
    (`SkeletalMeshComponent.PlayAnimation` (`self.DoorSK`) "/Game/VRTrueLocomotion/Meshes/Door/Anim_DoorClose.Anim_DoorClose" false)
    (set `self.IsDoorOpen` false)
    (`PrimitiveComponent.SetCollisionResponseToAllChannels` (`self.DoorSK`) "ECR_Block")))

(fn `UserConstructionScript`)