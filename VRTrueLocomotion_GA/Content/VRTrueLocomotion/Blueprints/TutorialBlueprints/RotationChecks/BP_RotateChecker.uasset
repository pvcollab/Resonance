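; BP_RotateChecker is a VR tutorial Blueprint that tracks completion of left and right rotation checks through two widget components.
; BeginPlay caches both check widgets and hides them, with show and hide events controlling each side's visibility.
; Tick polls each widget's throbber progress; when full, a DoOnce sets that side's completed flag, fires sparks and hides the widget after a short delay.
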(event `self.ReceiveBeginPlay`
  ;[0 1 0] EVENT BEGINPLAY
  (`|ExecutionSequence`
    (:`then_0`
      ;[1 1 1] Initial Cast to Rotation Checker Widgets
      (bind _asw_right_rotation_check (cast `/Game/VRTrueLocomotion/Blueprints/TutorialBlueprints/RotationChecks/W_RightRotationCheck` (`WidgetComponent.GetUserWidgetObject` (`self.W_RotatorRightCheck`))))
      (set `self.W_RightRotatorCheckRef` _asw_right_rotation_check)
      (bind _asw_left_rotation_check (cast `/Game/VRTrueLocomotion/Blueprints/TutorialBlueprints/RotationChecks/W_LeftRotationCheck` (`WidgetComponent.GetUserWidgetObject` (`self.W_RotatorLeftCheck`))))
      (set `self.W_LeftRotatorCheckRef` _asw_left_rotation_check))
    (:`then_1`
      ;[1 1 1] Initially Hides Left/Right Checkers
      (`self.CE_HidesLeftChecker`)
      (`self.CE_HidesRightChecker`))))

(event `self.ReceiveTick`
  (params (DeltaSeconds :type "Float (single-precision)"))
  ;[0 1 0] EVENT TICK
  (`|ExecutionSequence`
    (:`then_0`
      ;[1 1 1] Checks Right Throbber Progress/ Plays Sparks When Completed and Hides Itself
      (if (>= (`/Game/VRTrueLocomotion/Blueprints/TutorialBlueprints/RotationChecks/W_RightRotationCheck.ThrobberProgress` (`self.W_RightRotatorCheckRef`)) 1.0)
        (`/Engine/EditorBlueprintResources/StandardMacros.DoOnce` false
          (:`Completed`
            (set `self.CompletedRightRotCheck` true)
            (`ActorComponent.Activate` (`self.P_RightSparks`) false)
            (`KismetSystemLibrary.Delay` 0.5)
            (`self.CE_HidesRightChecker`)))))
    (:`then_1`
      ;[1 1 1] Checks Left Thobber Progess/ Plays Sparks When Completed and Hides Itself
      (if (>= (`/Game/VRTrueLocomotion/Blueprints/TutorialBlueprints/RotationChecks/W_LeftRotationCheck.ThrobberProgress` (`self.W_LeftRotatorCheckRef`)) 1.0)
        (`/Engine/EditorBlueprintResources/StandardMacros.DoOnce` false
          (:`Completed`
            (set `self.CompletedLeftRotCheck` true)
            (`ActorComponent.Activate` (`self.P_LeftSparks`) false)
            (`KismetSystemLibrary.Delay` 0.5)
            (`self.CE_HidesLeftChecker`)))))))

(event `CE_HidesRightChecker`
  ;[1 1 1] Right Checker Visibility
  (`SceneComponent.SetVisibility` (`self.W_RotatorRightCheck`) false true))

(event `CE_ShowsRightChecker`
  ;[1 1 1] Right Checker Visibility
  (`SceneComponent.SetVisibility` (`self.W_RotatorRightCheck`) true true))

(event `CE_HidesLeftChecker`
  ;[1 1 1] Right Checker Visibility
  (`SceneComponent.SetVisibility` (`self.W_RotatorLeftCheck`) false true))

(event `CE_ShowsLeftChecker`
  ;[1 1 1] Right Checker Visibility
  (`SceneComponent.SetVisibility` (`self.W_RotatorLeftCheck`) true true))

(fn `UserConstructionScript`)