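; VR locomotion component that drives the owning pawn by head movement: yaw turns, pitch walks or runs, roll strafes.
; A looping timer samples HMD orientation, and Tick applies each separately enabled axis while the headset is worn.
; Inputs are range-mapped and rescaled outside dead zones, with movement following camera forward and right vectors.
; Yaw is measured from an offset captured on first use, re-captured after locomotion is toggled off.
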(event `self.ReceiveBeginPlay`
  ;[0 1 0] BEGIN PLAY
  (`|ExecutionSequence`
    (:`then_0`
      ;[1 1 1] Set Reference To Owning Pawn
      (set `self.PawnReference` (`Actor.Instigator` (`self.GetOwner`))))
    (:`then_1`
      ;[1 1 1] Setting Custom Event Tick on Beginplay
      (`KismetSystemLibrary.K2_SetTimerDelegate` (delegate `CE_CustomEventTick`) (`self.CustomTickDelta`) true))
    (:`then_2`
      ;[1 1 1] Checking What HMD  is in Use
      (switch `name` (`HeadMountedDisplayFunctionLibrary.GetHMDDeviceName`)
        (:`Default`
          (set `self.IsOculusHMD` false :!label _label))
        (:`OculusHMD`
          (set `self.IsOculusHMD` true))
        (:`SteamVR`
          (goto _label))
        (:`PSVR`
          (goto _label))))))

(event `CE_TogglesMovement`
  ;[1 1 1] Toggle VR True Locomotion System
  (bind _output_get (set `self.EnableTrueLocomotion` (select `bool` (`self.EnableTrueLocomotion`) :`false` true)))
  (if (not _output_get)
    (`self.CE_ResetYawOffsetDo1`)))

(event `CE_CustomEventTick`
  ;[0 1 0] CUSTOM EVENT TICK
  ;[1 1 1] Get Current HMD Rotation
  (if (`self.IsOculusHMD`)
    (if (`|EnumEquality` (`HeadMountedDisplayFunctionLibrary.GetHMDWornState`) "Worn")
      (set `self.HMDCurrentYaw` (.yaw (`HeadMountedDisplayFunctionLibrary.GetOrientationAndPosition`)) :!label _label_2)
      (set `self.HMDCurrentPitch` (.pitch (`HeadMountedDisplayFunctionLibrary.GetOrientationAndPosition`)))
      (set `self.HMDCurrentRoll` (.roll (`HeadMountedDisplayFunctionLibrary.GetOrientationAndPosition`))))
    (else
      (goto _label_2))))

(event `CE_UpdatesYaw`
  ;[1 1 1] Turning
  ;;[1 1 1] Account for any initial camera rotation issues
  (`|ExecutionSequence`
    (:`then_0`
      (`/Engine/EditorBlueprintResources/StandardMacros.DoOnce` false :!label _label_3
        (:`Completed`
          (set `self.HMDYawOffset` (`self.HMDCurrentYaw`))
          (goto _label_4 :!via `Open`))))
    (:`then_1`
      (`/Engine/EditorBlueprintResources/StandardMacros.Gate` true :!label _label_4
        (:`Exit`
          (bind _output_get (set `self.ClampedYawInput` (`KismetMathLibrary.MapRangeClamped` (- (`self.HMDCurrentYaw`) (`self.HMDYawOffset`)) (`self.MinHMDYawRange`) (`self.MaxHMDYawRange`) -1.0 1.0)))
          (if (or (< _output_get (`self.YawLeftDeadZone`)) (> _output_get (`self.YawRightDeadZone`)))
            (bind _yawaxisinputvalue (`self.CalculateYawInputValue`))
            (`Pawn.AddControllerYawInput` (`self.PawnReference`) (* _yawaxisinputvalue (`self.YawInputMultiplier`)))))))))

(event `CE_ResetYawOffsetDo1`
  ;[1 1 1] Turning
  ;;[1 1 1] Account for any initial camera rotation issues
  (goto _label_3 :!via `Reset`))

(event `CE_UpdatesPitch`
  (bind _returnvalue (* (`KismetMathLibrary.MapRangeClamped` (`self.HMDCurrentPitch`) (`self.MinHMDPitchRange`) (`self.MaxHMDPitchRange`) -1.0 1.0) -1.0))
  ;[1 1 1] Walking/Running
  (bind _output_get (set `self.ClampedPitchInput` _returnvalue))
  (if (`KismetMathLibrary.NearlyEqual_FloatFloat` _returnvalue 0.0 0.0001)
    _
    (elif (or (> _output_get (`self.PitchFWDDeadZone`)) (< _output_get (`self.PitchBWDDeadZone`)))
      (bind _pitchaxisinputvalue (`self.CalculatePitchInputValue`))
      (`Pawn.AddMovementInput` (`self.PawnReference`) (`Actor.GetActorForwardVector` (`GameplayStatics.GetPlayerCameraManager` 0)) (* _pitchaxisinputvalue (`self.PitchInputMultiplier`)) false))))

(event `self.ReceiveTick`
  (params (DeltaSeconds :type "Float (single-precision)"))
  ;[0 1 0] NATIVE TICK
  ;[1 1 1] Update Yaw, Pitch, and Roll
  (if (`|EnumEquality` (`HeadMountedDisplayFunctionLibrary.GetHMDWornState`) "Worn")
    (if (`self.EnableTrueLocomotion`)
      (`|ExecutionSequence`
        (:`then_0`
          (if (`self.EnableVRTLTurning`)
            (`self.CE_UpdatesYaw`) ; Turn
          ))
        (:`then_1`
          (if (`self.EnableVRTLWalking/Running`)
            (`self.CE_UpdatesPitch`) ; Walk/Run
          ))
        (:`then_2`
          (if (`self.EnableVRTLStrafing`)
            (`self.CE_UpdateRoll`) ; Strafe
          ))))))

(event `CE_UpdateRoll`
  ;[1 1 1] Strafing
  (bind _output_get (set `self.ClampedRollInput` (`KismetMathLibrary.MapRangeClamped` (`self.HMDCurrentRoll`) (`self.MinHMDRollRange`) (`self.MaxHMDRollRange`) -1.0 1.0)))
  (if (`KismetMathLibrary.NearlyEqual_FloatFloat` _output_get 0.0 0.0001)
    _
    (elif (or (< _output_get (`self.RollLeftDeadZone`)) (> _output_get (`self.RollRightDeadZone`)))
      (bind _rollaxisinputvalue (`self.CalculateRollInputValue`))
      (`Pawn.AddMovementInput` (`self.PawnReference`) (`Actor.GetActorRightVector` (`GameplayStatics.GetPlayerCameraManager` 0)) (* _rollaxisinputvalue (`self.RollInputMultiplier`)) false))))

(fn `CalculatePitchInputValue`
  (returns (PitchAxisInputValue :type "Float (double-precision)"))
  (locals (PosMappedPitchInput :type "Float (double-precision)") (NegMappedPitchInput :type "Float (double-precision)"))
  (bind _clampedpitchinput (`self.ClampedPitchInput`))
  (bind _pitchbwddeadzone (`self.PitchBWDDeadZone`))
  (bind _pitchfwddeadzone (`self.PitchFWDDeadZone`))
  (`|ExecutionSequence`
    (:`then_0`
      (if (<= _clampedpitchinput _pitchbwddeadzone)
        (bind _output_get (set `local.NegMappedPitchInput` (`KismetMathLibrary.MapRangeClamped` _clampedpitchinput _pitchbwddeadzone -1.0 -0.001 -1.0)))
        (return _output_get)))
    (:`then_1`
      (if (>= _clampedpitchinput _pitchfwddeadzone)
        (bind _output_get_2 (set `local.PosMappedPitchInput` (`KismetMathLibrary.MapRangeClamped` _clampedpitchinput _pitchfwddeadzone 1.0 0.001 1.0)))
        (return _output_get_2)))))

(fn `CalculateRollInputValue`
  (returns (RollAxisInputValue :type "Float (double-precision)"))
  (locals (PosMappedRollInput :type "Float (double-precision)") (NegMappedRollInput :type "Float (double-precision)"))
  (bind _clampedrollinput (`self.ClampedRollInput`))
  (bind _rollrightdeadzone (`self.RollRightDeadZone`))
  (bind _rollleftdeadzone (`self.RollLeftDeadZone`))
  (`|ExecutionSequence`
    (:`then_0`
      (if (<= _clampedrollinput _rollleftdeadzone)
        (bind _output_get (set `local.NegMappedRollInput` (`KismetMathLibrary.MapRangeClamped` _clampedrollinput _rollleftdeadzone -1.0 -0.001 -1.0)))
        (return _output_get)))
    (:`then_1`
      (if (>= _clampedrollinput _rollrightdeadzone)
        (bind _output_get_2 (set `local.PosMappedRollInput` (`KismetMathLibrary.MapRangeClamped` _clampedrollinput _rollrightdeadzone 1.0 0.001 1.0)))
        (return _output_get_2)))))

(fn `CalculateYawInputValue`
  (returns (YawAxisInputValue :type "Float (double-precision)"))
  (locals (PosMappedYawInput :type "Float (double-precision)") (NegMappedYawInput :type "Float (double-precision)"))
  (bind _clampedyawinput (`self.ClampedYawInput`))
  (bind _yawleftdeadzone (`self.YawLeftDeadZone`))
  (bind _yawrightdeadzone (`self.YawRightDeadZone`))
  (`|ExecutionSequence`
    (:`then_0`
      (if (<= _clampedyawinput _yawleftdeadzone)
        (bind _output_get (set `local.NegMappedYawInput` (`KismetMathLibrary.MapRangeClamped` _clampedyawinput _yawleftdeadzone -1.0 -0.001 -1.0)))
        (return _output_get)))
    (:`then_1`
      (if (>= _clampedyawinput _yawrightdeadzone)
        (bind _output_get_2 (set `local.PosMappedYawInput` (`KismetMathLibrary.MapRangeClamped` _clampedyawinput _yawrightdeadzone 1.0 0.001 1.0)))
        (return _output_get_2)))))