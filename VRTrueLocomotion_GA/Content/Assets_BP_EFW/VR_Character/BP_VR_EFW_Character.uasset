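; BP_VR_EFW_Character is a VR player character that moves relative to where the right motion controller points.
; On BeginPlay it adds the right-hand Enhanced Input mapping context and calls a zero-velocity LaunchCharacter with XY override.
; Legacy MovementAxisRight X and Y axis events feed AddMovementInput along the controller's right and forward vectors.
; The VRTL_MovementFWD axis event is an empty stub.
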(event `InputAxis|VRTL_MovementFWD`
  (params (AxisValue :type "Float (single-precision)")))

(event `self.ReceiveBeginPlay`
  (bind _asplayer_controller (cast `PlayerController` (`self.GetController`)))
  (message `EnhancedInputSubsystemInterface.AddMappingContext` (pcsubsystem `EnhancedInputLocalPlayerSubsystem` _asplayer_controller) "/Game/Assets_BP_EFW/VR_Character/EFW_InputMappingContext_Right.EFW_InputMappingContext_Right" 0 (struct))
  (`self.LaunchCharacter` (0.0 0.0 0.0) true))

(event `InputAxis|MovementAxisRight_X`
  (params (AxisValue :type "Float (single-precision)"))
  (`self.AddMovementInput` (`SceneComponent.GetRightVector` (`self.MotionControllerRight`)) AxisValue))

(event `InputAxis|MovementAxisRight_Y`
  (params (AxisValue :type "Float (single-precision)"))
  (`self.AddMovementInput` (`SceneComponent.GetForwardVector` (`self.MotionControllerRight`)) AxisValue))

(fn `UserConstructionScript`)